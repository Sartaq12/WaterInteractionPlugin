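; Oceanology Infinity ocean variant for FluidNinja that re-applies the ocean's parameters to its materials at play start.
; BeginPlay runs the parent, waits briefly so the ninja material sync finishes, then runs InitializeParamsOnly, LandscapeModulator and LocationOffset.
; InitializeParamsOnly re-fetches the WaterPreviewGrid material as OceanSurface, then macros push settings structs into MPC_Waves, near and far surface materials, underwater post-process and god-ray materials.
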(event EventBeginPlay
  (|CallParentFunction)
  ;[1 1 1] This is necessary to sync up Oceanology parameters after ninja material sync.
  (Utilities|FlowControl|Delay 0.1)
  (CallFunction|InitializeParamsOnly)
  (CallFunction|LandscapeModulator)
  (CallFunction|LocationOffset))

(fn ConstructionScript
  (|CallParentFunction))

(fn InitializeParamsOnly
  (Variables|Default|SetOcean%20surface (.AsMaterial%20Instance%20Dynamic (Utilities|Casting|CastToMaterialInstanceDynamic (Rendering|Material|GetMaterial (Variables|Default|GetWaterPreviewGrid) 0))))
  ;[0 0 0 1 100] Gerstner Waves
  (|GerstnerWaves(Parameters)_2)
  ;[0 0 0 1 100] Underwater
  (|Underwater(Parameters)_2)
  ;[0 0 0 1 100] God Rays
  (|GodRays(Parameters)_2)
  ;[0 0 0 1 100] caustic system
  (|CausticSystem_2)
  ;[0 0 0 1 100] Shoreline Interaction
  (|ShorelineInteraction(Parameters)_2)
  ;[0 0 0 1 100] Surface Light
  (|SurfaceLight(Parameters)_2)
  ;[0 0 0 1 100] Advanced Foam Generator
  (|AdvancedFoamGenerator(Parameters)_2)
  ;[0 0 0 1 100] Refraction
  (|Refraction(Parameters)_2)
  ;[0 0 0 1 100] Normal
  (|Normal(Parameters)_2))